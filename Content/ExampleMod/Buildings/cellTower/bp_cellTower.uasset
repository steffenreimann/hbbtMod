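; Cell tower building Blueprint that keeps a record of the user phones connecting to it.
; On BeginPlay it binds a handler to its UserPhoneConnect event, which adds the caller to the ConnectedPhone array if absent.
; The handler then casts the caller and calls its CBuserPhoneConnectEvent with the tower as argument, acting as a connection callback.
; NetFuncTest is an empty stub.
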(event Custom|userPhoneConnect_Event
  (params (from :type Object%20Object%20Reference))
  (CallFunction|CheckUser from)
  (bind _assmartphone (Utilities|Casting|CastTo from))
  (CallFunction|CBuserPhoneConnectEvent _assmartphone self))

(event EventBeginPlay
  (EventDispatchers|BindEventtoUserPhoneConnect (delegate Custom|userPhoneConnect_Event)))

(event Collision|EventActorBeginOverlap
  (params (OtherActor :type Actor%20Object%20Reference)))

(event EventTick
  (params (DeltaSeconds :type Float%20%28single-precision%29)))

(fn ConstructionScript)

(fn NetFuncTest
  (return))

(fn CheckUser
  (params (NewParam :type Object%20Object%20Reference))
  (bind _connectedphone (Variables|Default|GetconnectedPhone))
  (bind _returnvalue (Utilities|Array|FindItem _connectedphone NewParam))
  (if (== _returnvalue -1)
    (bind _returnvalue_2 (Utilities|Array|Add _connectedphone NewParam))
    (return _returnvalue_2)
    (else
      (return _returnvalue))))