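; Remote link actor in ExampleMod that watches a connected building's storage and notifies smartphones when its contents change.
; On begin play it resolves the building type and typed references, and caches initial overlay info for storage.
; A once-per-second tick polls storage info for any connected type, compares it to the cache, and calls the storage-change event on every smartphone's interact widget.
; Factory, miner and generator info queries are unwired.
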(event Collision|EventActorBeginOverlap
  (params (OtherActor :type Actor%20Object%20Reference)))

(event EventBeginPlay
  (Actor|Tick|SetActorTickEnabled true)
  (Actor|Tick|SetActorTickInterval 1.0)
  (bind (_newparam _asfgbuildable_factory _asfgbuildable_manufacturer _asfgbuildable_storage _asfgcrate _asfgbuildable_resource_extractor _asfgbuildable_generator) (Default|GetBuildingType (Variables|Components|Getlib) (Variables|Default|GetConnectedActor)))
  (bind _output_get (Variables|Default|SetbuildingType _newparam))
  (Variables|Default|SetFactory _asfgbuildable_factory)
  (Variables|Default|SetManufactur _asfgbuildable_manufacturer)
  (Variables|Default|SetStorage _asfgbuildable_storage)
  (Variables|Default|SetCrate _asfgcrate)
  (Variables|Default|SetMiner _asfgbuildable_resource_extractor)
  (Variables|Default|SetGenerator _asfgbuildable_generator)
  (switch Utilities|FlowControl|Switch|SwitchonbuildingType _output_get
    (:NewEnumerator1
      (bind _overlayinfo (Default|GetStorageInfo (Variables|Components|Getlib) (Variables|Default|GetConnectedActor)))
      (Variables|Default|Setcurrent _overlayinfo))))

(event EventTick
  (params (DeltaSeconds :type Float%20%28single-precision%29))
  (bind _overlayinfo (Default|GetStorageInfo (Variables|Components|Getlib) (Variables|Default|GetConnectedActor)))
  (if (not (Utilities|Array|Identical _overlayinfo (Variables|Default|Getcurrent)))
    (Variables|Default|Setcurrent _overlayinfo)
    (bind _outactors (Actor|GetAllActorsOfClass "/Game/ExampleMod/Handables/smartphone/bp_smartphone.bp_smartphone_C"))
    (for _array_element _outactors
      (Default|CallOnStorageChange (Variables|/Game/ExampleMod/Handables/smartphone/bp_smartphone.bp_smartphone_C|Getwg_smartphone_interact _array_element)))))

(fn ConstructionScript)