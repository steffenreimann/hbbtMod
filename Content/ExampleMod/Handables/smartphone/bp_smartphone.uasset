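; Equippable smartphone that links the player to a radio tower and serves as the access point for its network UI.
; Equipping shows a HUD widget; primary fire camera-traces for a tower to request a connection, or opens the interaction widget with mouse input once connected.
; Event bindings made at BeginPlay record the connected tower, store custom UI panels and network data on the phone, and relay them to that widget.
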(event Custom|CBuserPhoneConnect_Event
  (params (NewParam :type Object%20Object%20Reference))
  ;[1 1 1] Event Begin Play Init
  (Variables|Default|SetConnectedTower NewParam)
  (Variables|Default|Setconnected? true)
  (Class|SMLBlueprintLibrary|LogDebug (Utilities|String|ToString(Text) (Utilities|Text|FormatText "Smartphone connected to {0}" (Utilities|Text|ToText(String) (Utilities|GetDisplayName NewParam)))) true))

(event Custom|setConnection_Event
  (params (NewParam :type Object%20Object%20Reference))
  ;[1 1 1] Event Begin Play Init
  (Class|SMLBlueprintLibrary|LogDebug "EquipSmartphone setConnection Event" true))

(event Custom|wg_sendToSmartphone_Event
  (params (NewParam :type String))
  ;[1 1 1] Event Begin Play Init
  (Class|SMLBlueprintLibrary|LogDebug (Utilities|String|ToString(Text) (Utilities|Text|FormatText "Smartphone .. get Data from Widget= {0}" (Utilities|Text|ToText(String) NewParam))) true))

(event Custom|savePanels_Event
  (params (NewParam :type Array%20of%20Struct%20Custom%20UI%20Structures))
  ;[1 1 1] Save Panels to Smartphone
  (Variables|Default|SetcustomUIPanels NewParam)
  (Class|SMLBlueprintLibrary|LogDebug "Save Panels to Smartphone" true))

(event Custom|getPanels_Event
  ;[1 1 1] get Panel from Smartphone
  (Default|CallGetPanelstoUI (Variables|Default|Getwg_smartphone_interact) (Variables|Default|GetcustomUIPanels))
  (Class|SMLBlueprintLibrary|LogDebug "send Panels to UI" true))

(event Custom|sendNetworkDataToSmartphone_Event
  ;[1 1 1] Event send Network Data to UI
  (Default|GetDatafromSmartphoneEvent (Variables|Default|Getwg_smartphone_interact) (Variables|Default|GetNetworkData)))

(event Custom|getDataFromNetwork_Event
  (params (NetData :type Array%20of%20Struct%20Network%20Data%20Structures))
  ;[1 1 1] get Data from Network and send to UI
  (bind _output_get (Variables|Default|SetNetworkData NetData))
  (Default|GetDatafromSmartphoneEvent (Variables|Default|Getwg_smartphone_interact) _output_get))

(event EventBeginPlay
  ;[1 1 1] Event Begin Play Init
  (EventDispatchers|BindEventtoSetConnection (delegate Custom|setConnection_Event))
  (EventDispatchers|BindEventtoCBuserPhoneConnect (delegate Custom|CBuserPhoneConnect_Event))
  (EventDispatchers|BindEventtoWgSendtoSmartphone (delegate Custom|wg_sendToSmartphone_Event))
  (Class|SMLBlueprintLibrary|LogDebug "EquipSmartphone BeginPlay" true)
  ;[1 1 1] Save Panels to Smartphone
  (EventDispatchers|BindEventtoSavePanelstoSmartphone (delegate Custom|savePanels_Event))
  ;[1 1 1] get Panel from Smartphone
  (EventDispatchers|BindEventtoGetPanelsfromSmartphone (delegate Custom|getPanels_Event))
  ;[1 1 1] get Data from Network and send to UI
  (EventDispatchers|BindEventtoGetDatafromNetwork (delegate Custom|getDataFromNetwork_Event))
  ;[1 1 1] Write Player Ref to Var
  (bind _asfgcharacter_player (Utilities|Casting|CastToFGCharacterPlayer (Game|GetPlayerCharacter 0)))
  (Variables|Default|Setplayer _asfgcharacter_player)
  ;[1 1 1] Event send Network Data to UI
  (EventDispatchers|BindEventtoSendNetworkDatatoSmartphone (delegate Custom|sendNetworkDataToSmartphone_Event)))

(event Collision|EventActorBeginOverlap
  (params (OtherActor :type Actor%20Object%20Reference)))

(event EventTick
  (params (DeltaSeconds :type Float%20%28single-precision%29)))

(event EventWasEquipped
  (bind _returnvalue (Game|GetPlayerController 0))
  (Class|SMLBlueprintLibrary|LogDebug "Smartphone was Equipped" true)
  (Class|SMLBlueprintLibrary|LogDebug (Utilities|String|ToString(Text) (Utilities|Text|FormatText "get Player Controller {0} // get Owning Player {1}" (Utilities|Text|ToText(String) (Utilities|GetDisplayName _returnvalue)))))
  (bind _returnvalue_2 (UserInterface|CreateWidget "/Game/ExampleMod/Handables/smartphone/widgets/Overlay/wg_smartphone.wg_smartphone_C" _returnvalue))
  (bind _output_get (Variables|Default|Setwg_smartphone _returnvalue_2))
  (UserInterface|Viewport|AddtoViewport _output_get -1)
  (Class|SMLBlueprintLibrary|LogDebug "Widget add to Viewport" true)
  (Rendering|Components|TextRender|SetText (Variables|/Game/ExampleMod/Handables/smartphone/widgets/Overlay/wg_smartphone.wg_smartphone_C|GetbpText _output_get) "Equip Smartphone!"))

(event EventWasUnEquipped
  (Widget|RemovefromParent (stale EventWasEquipped _output_get))
  (Class|SMLBlueprintLibrary|LogDebug "Widget removed form parent" true))

(event EventDoDefaultPrimaryFire
  (bind _returnvalue (Game|GetPlayerController 0))
  (Class|SMLBlueprintLibrary|LogDebug "Primary Fire " true)
  (if (Variables|Default|Getconnected?)
    (Input|SetInputModeUIOnly _returnvalue (Variables|Default|Getwg_smartphone) "DoNotLock")
    (Variables|/Script/Engine.PlayerController|SetbShowMouseCursor _returnvalue true)
    (bind _returnvalue_2 (UserInterface|CreateWidget "/Game/ExampleMod/Handables/smartphone/widgets/IteractUI/wg_smartphoneInteract.wg_smartphoneInteract_C" _returnvalue self (Variables|Default|Getlast_view) 0 0 (Variables|Default|GetcustomUIPanels)))
    (bind _output_get (Variables|Default|Setwg_smartphone_interact _returnvalue_2))
    (UserInterface|Viewport|AddtoViewport _output_get 0)
    (else
      (bind (_hitactor _returnvalue_3) (CallFunction|Trace (Variables|Default|Getplayer) "/Game/ExampleMod/Buildings/cellTower/bp_radiotower.bp_radiotower_C"))
      (if _returnvalue_3
        (bind _asbp_radiotower (Utilities|Casting|CastTobp_radiotower _hitactor))
        (Default|UserPhoneConnectEvent _asbp_radiotower self)))))

(fn ConstructionScript)

(fn Trace
  (params (Player :type FG%20Character%20Player%20Object%20Reference) (B :type Object%20Class%20Reference))
  (bind _returnvalue (Class|FGCharacterPlayer|GetCameraComponent Player))
  (bind _returnvalue_2 (Transformation|GetWorldLocation _returnvalue))
  (bind _outhit (Collision|LineTraceByChannel _returnvalue_2 (+ _returnvalue_2 (* (Math|Vector|GetForwardVector (Transformation|GetWorldRotation _returnvalue)) 1.5e+03)) "TraceTypeQuery1" false 0 "ForDuration"))
  (return (.HitActor (Collision|BreakHitResult _outhit)) (== (Utilities|GetClass (.HitActor (Collision|BreakHitResult _outhit))) B)))

(fn BuildSPUI)

(fn BuildSPUIopen)

(fn InitPanels)

(fn RefreshData
  (params (New%20Data :type Array%20of%20Struct%20Network%20Data%20Structures) (Old%20Data :type Array%20of%20Struct%20Network%20Data%20Structures))
  (Class|SMLBlueprintLibrary|LogDebug "Smartphone Refresh Data " true)
  (for _array_element New%20Data
    (if (== (Utilities|Array|FindItem Old%20Data _array_element) -1)
      (Utilities|Array|Add Old%20Data _array_element)
      (else
        (Utilities|Array|SetArrayElem Old%20Data (Utilities|Array|FindItem Old%20Data _array_element) _array_element))))
  (return))