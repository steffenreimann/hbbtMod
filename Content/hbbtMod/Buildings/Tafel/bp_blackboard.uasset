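; Blackboard building actor that carries a UMG widget through its Widget component.
; On BeginPlay it runs the parent logic, then casts the component's user widget to wg_blackboard_world and caches it as WorldWidget.
; It has no other logic of its own: overlap and tick events are disabled, and the construction script only calls its parent.
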(event EventBeginPlay
  (|CallParentFunction)
  (bind _aswg_blackboard_world (Utilities|Casting|CastTowg_blackboard_world (UserInterface|GetUserWidgetObject (Variables|Default|GetWidget))))
  (Variables|Default|SetWorldWidget _aswg_blackboard_world))

(event Collision|EventActorBeginOverlap
  (params (OtherActor :type Actor%20Object%20Reference))
  (|CallParentFunction OtherActor) ; This node is disabled and will not be called.\nDrag off pins to build functionality.
)

(event EventTick
  (params (DeltaSeconds :type Float%20%28single-precision%29))
  (|CallParentFunction DeltaSeconds) ; This node is disabled and will not be called.\nDrag off pins to build functionality.
)

(fn ConstructionScript
  (|CallParentFunction))