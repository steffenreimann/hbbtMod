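; Placeable blackboard (Tafel) building that shows editable multi-line text on a world widget inside a movable frame.
; BeginPlay caches the widget, binds move, rotate, scale and text events, then applies string-defined text/background colors and frame visibility.
; Handlers offset the frame relative to its current transform, set absolute scale, or update text and a hard-coded text style.
; Interval Tick only logs; transform-restore and miner/generator info logic is unconnected.
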(event Custom|scaleInfo_Event
  (params (scale :type Vector))
  (bind _output_get (Variables|Default|Setscale (+ scale (Transformation|GetWorldScale (Variables|Default|GetFrame)))))
  (Transformation|SetWorldScale3D (Variables|Default|GetFrame) _output_get))

(event Custom|moveInfo_Event
  (params (distance :type Float%20%28single-precision%29) (direction :type Rotator))
  (bind _frame (Variables|Default|GetFrame))
  (bind _returnvalue (Transformation|GetWorldRotation _frame))
  (bind (_roll _pitch _yaw) (Math|Rotator|BreakRotator _returnvalue))
  ;[1 1 1] Comment
  (Variables|Default|Setdistance distance)
  (Variables|Default|Setdirection direction)
  (Class|SMLBlueprintLibrary|LogDebug (Utilities|String|ToString(Vector) (* (Math|Vector|GetForwardVector (Math|Rotator|MakeRotator (+ _roll (.Roll (Math|Rotator|BreakRotator (Variables|Default|Getdirection)))) (+ _pitch (.Pitch (Math|Rotator|BreakRotator (Variables|Default|Getdirection)))) (+ _yaw (.Yaw (Math|Rotator|BreakRotator (Variables|Default|Getdirection)))))) (Variables|Default|Getdistance))) true)
  (Transformation|SetWorldLocation (Variables|Default|GetFrame) (+ (Transformation|GetWorldLocation (Variables|Default|GetFrame)) (* (Math|Vector|GetForwardVector (Math|Rotator|MakeRotator (+ _roll (.Roll (Math|Rotator|BreakRotator (Variables|Default|Getdirection)))) (+ _pitch (.Pitch (Math|Rotator|BreakRotator (Variables|Default|Getdirection)))) (+ _yaw (.Yaw (Math|Rotator|BreakRotator (Variables|Default|Getdirection)))))) (Variables|Default|Getdistance))) false false)
  (Variables|Default|Setlocation (+ (Transformation|GetWorldLocation (Variables|Default|GetFrame)) (* (Math|Vector|GetForwardVector (Math|Rotator|MakeRotator (+ _roll (.Roll (Math|Rotator|BreakRotator (Variables|Default|Getdirection)))) (+ _pitch (.Pitch (Math|Rotator|BreakRotator (Variables|Default|Getdirection)))) (+ _yaw (.Yaw (Math|Rotator|BreakRotator (Variables|Default|Getdirection)))))) (Variables|Default|Getdistance))))
  (Class|SMLBlueprintLibrary|LogDebug "event move"))

(event Custom|changeText_Event
  (params (Text :type Text))
  ;[1 0.4061 0] Comment
  (Class|SMLBlueprintLibrary|LogDebug "change Text" true)
  (Class|SMLBlueprintLibrary|LogDebug (Utilities|String|ToString(Text) Text) true)
  (Rendering|Components|TextRender|SetText (Variables|/Game/hbbtMod/Buildings/Tafel/wg_blackboard_world.wg_blackboard_world_C|GetMultiLineEditableTextBox_47 (Variables|Default|GetWorldWirdget)) Text))

(event Custom|rotateInfo_Event
  (params (rot :type Rotator))
  (bind (_roll _pitch _yaw) (Math|Rotator|BreakRotator rot))
  (bind _frame (Variables|Default|GetFrame))
  (bind _returnvalue (Transformation|GetWorldRotation _frame))
  (bind (_roll_2 _pitch_2 _yaw_2) (Math|Rotator|BreakRotator _returnvalue))
  (bind _returnvalue_2 (+ _roll_2 _roll))
  (bind _returnvalue_3 (+ _pitch_2 _pitch))
  (bind _returnvalue_4 (+ _yaw_2 _yaw))
  (bind _returnvalue_5 (Math|Rotator|MakeRotator _returnvalue_2 _returnvalue_3 _returnvalue_4))
  ;[1 1 1] Comment
  (Variables|Default|Setrotation _returnvalue_5)
  (Transformation|SetWorldRotation (Variables|Default|GetFrame) _returnvalue_5 false false))

(event Custom|changeTextStyle_Event
  (bind _output_get (Variables|/Script/UMG.MultiLineEditableTextBox|SetTextStyle (Variables|/Game/hbbtMod/Buildings/Tafel/wg_blackboard_world.wg_blackboard_world_C|GetMultiLineEditableTextBox_47 (Variables|Default|GetWorldWirdget)) (Utilities|Struct|MakeTextBlockStyle (Utilities|Struct|MakeSlateFontInfo 0 0 (Utilities|Struct|MakeFontOutlineSettings 0 false)) (Utilities|Struct|MakeSlateColor "(R=1.000000,G=0.000000,B=1.000000,A=1.000000)") "(X=0.000000,Y=0.000000)" "(R=0.000000,G=0.000000,B=0.000000,A=1.000000)")))
  (Variables|Text|SetText%20Style _output_get))

(event Custom|setScale_Event
  (params (NewParam :type Vector))
  (Transformation|SetWorldScale3D (Variables|Default|GetFrame) NewParam))

(event EventBeginPlay
  (Class|SMLBlueprintLibrary|LogDebug "Begin Play on Tafel !!!!!!!!" true)
  (bind _aswg_blackboard_world (Utilities|Casting|CastTowg_blackboard_world (UserInterface|GetUserWidgetObject (Variables|Default|GetWidget))))
  (Variables|Default|SetWorldWirdget _aswg_blackboard_world)
  ;[1 1 1] Enable Tick and set Interval
  (Actor|Tick|SetActorTickEnabled true)
  (Actor|Tick|SetActorTickInterval (Variables|Default|GetactorTick))
  (EventDispatchers|BindEventtoDoMove (delegate Custom|moveInfo_Event))
  (EventDispatchers|BindEventtoDoRotate (delegate Custom|rotateInfo_Event))
  (EventDispatchers|BindEventtoDoScale (delegate Custom|scaleInfo_Event))
  (EventDispatchers|BindEventtoSetScale (delegate Custom|setScale_Event))
  (EventDispatchers|BindEventtoChangeText (delegate Custom|changeText_Event))
  (EventDispatchers|BindEventtoChangeTextStyle (delegate Custom|changeTextStyle_Event))
  ;[1 1 1] on Game Start
  ;;[1 1 1] Set Text Color
  (bind _slatecolor (Default|MakeSlateColorwithString (Variables|Default|Getlib) (Variables|Text|GetTextColorString)))
  (bind _structout (Utilities|Struct|SetmembersinEditableTextBoxStyle (Variables|/Script/UMG.MultiLineEditableTextBox|GetWidgetStyle (Variables|/Game/hbbtMod/Buildings/Tafel/wg_blackboard_world.wg_blackboard_world_C|GetMultiLineEditableTextBox_47 (Variables|Default|GetWorldWirdget))) _slatecolor))
  (Variables|/Script/UMG.MultiLineEditableTextBox|SetWidgetStyle (Variables|/Game/hbbtMod/Buildings/Tafel/wg_blackboard_world.wg_blackboard_world_C|GetMultiLineEditableTextBox_47 (Variables|Default|GetWorldWirdget)) _structout)
  ;;[1 1 1] Set Background Color
  (bind _slatecolor_2 (Default|MakeSlateColorwithString (Variables|Default|Getlib) (Variables|Text|GetBackgroundColorString)))
  (bind _structout_2 (Utilities|Struct|SetmembersinEditableTextBoxStyle (Variables|/Script/UMG.MultiLineEditableTextBox|GetWidgetStyle (Variables|/Game/hbbtMod/Buildings/Tafel/wg_blackboard_world.wg_blackboard_world_C|GetMultiLineEditableTextBox_47 (Variables|Default|GetWorldWirdget))) _slatecolor_2))
  (Variables|/Script/UMG.MultiLineEditableTextBox|SetWidgetStyle (Variables|/Game/hbbtMod/Buildings/Tafel/wg_blackboard_world.wg_blackboard_world_C|GetMultiLineEditableTextBox_47 (Variables|Default|GetWorldWirdget)) _structout_2)
  ;;[1 1 1] set Visablility
  (if (Variables|Text|GetFrameShow)
    (Rendering|SetVisibility (Variables|Default|GetFrame) true false)
    (else
      (Rendering|SetVisibility (Variables|Default|GetFrame) false false))))

(event Collision|EventActorBeginOverlap
  (params (OtherActor :type Actor%20Object%20Reference)))

(event EventTick
  (params (DeltaSeconds :type Float%20%28single-precision%29))
  (Class|SMLBlueprintLibrary|LogDebug "Tafel Event Tick !!!!!!!!" true))

(fn ConstructionScript)