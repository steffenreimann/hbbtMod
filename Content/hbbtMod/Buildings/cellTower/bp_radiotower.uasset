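; Radio tower Blueprint that acts as a cell network hub, registering smartphones and relaying data to them.
; On BeginPlay it binds network events, flags stored phones as connected and drops invalid entries; new connections are added once and get a callback with the tower.
; Its send function parses incoming data, refreshes a network buffer and broadcasts the result to every connected phone.
; The get-network-data handler is an empty stub.
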(event Custom|userPhoneConnect_Event
  (params (NewParam :type Object%20Object%20Reference))
  (bind _connectedphone (Variables|Default|GetconnectedPhone))
  (if (== (Utilities|Array|FindItem _connectedphone NewParam) -1)
    (Utilities|Array|Add _connectedphone NewParam)
    (bind _asbp_smartphone (Utilities|Casting|CastTobp_smartphone NewParam))
    (Default|CBuserPhoneConnectEvent _asbp_smartphone self)))

(event Custom|getNetworkData_Event)

(event EventBeginPlay
  (bind _connectedphone (Variables|Default|GetconnectedPhone))
  (EventDispatchers|BindEventtoUserPhoneConnect (delegate Custom|userPhoneConnect_Event))
  (EventDispatchers|BindEventtoGetNetworkData (delegate Custom|getNetworkData_Event))
  (for (_array_element _array_index) _connectedphone
    (bind _asbp_smartphone (Utilities|Casting|CastTobp_smartphone _array_element)
      (:then
        (Variables|/Game/hbbtMod/Handables/smartphone/bp_smartphone.bp_smartphone_C|Setconnected? _asbp_smartphone true))
      (:CastFailed
        (Utilities|Array|RemoveIndex _connectedphone _array_index)))))

(event Collision|EventActorBeginOverlap
  (params (OtherActor :type Actor%20Object%20Reference)))

(event EventTick
  (params (DeltaSeconds :type Float%20%28single-precision%29)))

(fn ConstructionScript)

(fn NetFuncPhoneLog
  (params (NewParam :type String))
  (Class|SMLBlueprintLibrary|LogDebug NewParam true))

(fn NetFuncSendData
  (params (NewParam :type String))
  (bind _lib (Variables|Default|Getlib))
  (Class|SMLBlueprintLibrary|LogDebug NewParam true)
  (bind _netdata (Default|Parse _lib NewParam))
  (Default|RefreshArray _lib _netdata (Variables|Default|GetNetDataBuffer))
  (for (_array_element _array_index) (Variables|Default|GetconnectedPhone)
    (bind _asbp_smartphone (Utilities|Casting|CastTobp_smartphone _array_element)
      (:then
        (Default|CallGetDatafromNetwork _asbp_smartphone _netdata)
        (Class|SMLBlueprintLibrary|LogDebug "Data sended" true))
      (:CastFailed
        (Class|SMLBlueprintLibrary|LogDebug "netFunc_SendData cant cast to Smartphone" true))))
  (return "netFunc_SendData" _array_index))