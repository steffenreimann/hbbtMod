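; World info display actor that shows factory, storage, miner or generator details for buildings on UMG widgets.
; BeginPlay restores or saves the Cube1 transform and binds move, rotate and scale events that adjust and store it.
; A five-second Tick loops over Refcatch, rebuilding widgets by building type from ContainerActor data; storage gets a sorted, truncated list with an item total.
; The master and container widget setup is disconnected and never runs.
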(event Custom|scaleInfo_Event
  (params (scale :type Vector))
  (bind _output_get (Variables|Default|Setscale (+ scale (Transformation|GetWorldScale (Variables|Default|GetCube1)))))
  (Transformation|SetWorldScale3D (Variables|Default|GetCube1) _output_get))

(event Custom|moveInfo_Event
  (params (distance :type Float%20%28single-precision%29) (direction :type Rotator))
  (bind _cube1 (Variables|Default|GetCube1))
  (bind _returnvalue (Transformation|GetWorldRotation _cube1))
  (bind (_roll _pitch _yaw) (Math|Rotator|BreakRotator _returnvalue))
  ;[1 1 1] Comment
  (Variables|Default|Setdistance distance)
  (Variables|Default|Setdirection direction)
  (Class|SMLBlueprintLibrary|LogDebug (Utilities|String|ToString(Vector) (* (Math|Vector|GetForwardVector (Math|Rotator|MakeRotator (+ _roll (.Roll (Math|Rotator|BreakRotator (Variables|Default|Getdirection)))) (+ _pitch (.Pitch (Math|Rotator|BreakRotator (Variables|Default|Getdirection)))) (+ _yaw (.Yaw (Math|Rotator|BreakRotator (Variables|Default|Getdirection)))))) (Variables|Default|Getdistance))) true)
  (Transformation|SetWorldLocation (Variables|Default|GetCube1) (+ (Transformation|GetWorldLocation (Variables|Default|GetCube1)) (* (Math|Vector|GetForwardVector (Math|Rotator|MakeRotator (+ _roll (.Roll (Math|Rotator|BreakRotator (Variables|Default|Getdirection)))) (+ _pitch (.Pitch (Math|Rotator|BreakRotator (Variables|Default|Getdirection)))) (+ _yaw (.Yaw (Math|Rotator|BreakRotator (Variables|Default|Getdirection)))))) (Variables|Default|Getdistance))) false false)
  (Variables|Default|Setlocation (+ (Transformation|GetWorldLocation (Variables|Default|GetCube1)) (* (Math|Vector|GetForwardVector (Math|Rotator|MakeRotator (+ _roll (.Roll (Math|Rotator|BreakRotator (Variables|Default|Getdirection)))) (+ _pitch (.Pitch (Math|Rotator|BreakRotator (Variables|Default|Getdirection)))) (+ _yaw (.Yaw (Math|Rotator|BreakRotator (Variables|Default|Getdirection)))))) (Variables|Default|Getdistance))))
  (Class|SMLBlueprintLibrary|LogDebug "event move"))

(event Custom|rotateInfo_Event
  (params (rot :type Rotator))
  (bind (_roll _pitch _yaw) (Math|Rotator|BreakRotator rot))
  (bind _cube1 (Variables|Default|GetCube1))
  (bind _returnvalue (Transformation|GetWorldRotation _cube1))
  (bind (_roll_2 _pitch_2 _yaw_2) (Math|Rotator|BreakRotator _returnvalue))
  (bind _returnvalue_2 (+ _roll_2 _roll))
  (bind _returnvalue_3 (+ _pitch_2 _pitch))
  (bind _returnvalue_4 (+ _yaw_2 _yaw))
  (bind _returnvalue_5 (Math|Rotator|MakeRotator _returnvalue_2 _returnvalue_3 _returnvalue_4))
  ;[1 1 1] Comment
  (Variables|Default|Setrotation _returnvalue_5)
  (Transformation|SetWorldRotation (Variables|Default|GetCube1) _returnvalue_5 false false))

(event EventBeginPlay
  (bind _transform (Variables|Default|GetTransform))
  (bind (_location _rotation) (Math|Transform|BreakTransform _transform))
  (Utilities|FlowControl|Sequence
    (:then_0
      ;[1 1 1] Comment
      (if (Math|Vector|Equal(Vector) (Variables|Default|Getlocation) "0, 0, 0" 0.0001)
        (Variables|Default|Setlocation _location)
        (Variables|Default|Setrotation _rotation))
      (Transformation|SetWorldLocationAndRotation (Variables|Default|GetCube1) (Variables|Default|Getlocation) (Variables|Default|Getrotation) false false)
      (Transformation|SetWorldScale3D (Variables|Default|GetCube1) (Variables|Default|Getscale)))
    (:then_1
      ;[1 1 1] Enable Tick and set Interval
      (Actor|Tick|SetActorTickEnabled true)
      (Actor|Tick|SetActorTickInterval 5.0)
      (EventDispatchers|BindEventtoMoveInfo (delegate Custom|moveInfo_Event))
      (EventDispatchers|BindEventtoRotateInfo (delegate Custom|rotateInfo_Event))
      (EventDispatchers|BindEventtoScaleInfo (delegate Custom|scaleInfo_Event)))))

(event Collision|EventActorBeginOverlap
  (params (OtherActor :type Actor%20Object%20Reference)))

(event EventTick
  (params (DeltaSeconds :type Float%20%28single-precision%29))
  (bind _lib (Variables|Default|Getlib))
  ;[0.2722 0 1] Comment
  (for _array_element (Variables|Default|Getrefcatch)
    (bind _newparam (Default|GetBuildingType (Variables|Default|Getlib) _array_element))
    (Utilities|Array|Add (Variables|Default|GetbuildingType) _newparam)
    (switch Utilities|FlowControl|Switch|SwitchonbuildingType _newparam
      (:NewEnumerator0
        ;[1 1 1] Comment
        (Widget|Panel|ClearChildren (Variables|/Game/hbbtMod/Handables/smartphone/widgets/world/wg_MasterInfo.wg_MasterInfo_C|GetCanvasPanel_0 (Variables|Default|GetMasterWidget)))
        (bind (_factoryinfo _cast) (Default|GetFactoryInfo (Variables|Default|Getlib) (Variables|Default|GetcontainerActor)))
        (if _cast
          (bind _returnvalue (UserInterface|CreateWidget "/Game/hbbtMod/Handables/smartphone/widgets/world/Factory/wg_FactoryInfo.wg_FactoryInfo_C" 0 _factoryinfo))
          (Class|CanvasPanel|AddChildtoCanvas (Variables|/Game/hbbtMod/Handables/smartphone/widgets/world/wg_MasterInfo.wg_MasterInfo_C|GetCanvasPanel_0 (Variables|Default|GetMasterWidget)) _returnvalue)
          (else
            (Class|SMLBlueprintLibrary|LogDebug "cant cast destroy actor -----------" true))))
      (:NewEnumerator1
        ;[1 1 1] Comment
        (Widget|Panel|ClearChildren (Variables|/Game/hbbtMod/Handables/smartphone/widgets/world/Storage/wg_containerInfo.wg_containerInfo_C|GetVerticalBox_70 (Variables|Default|GetContaionerInfo)))
        (bind (_overlayinfo _cast_2) (Default|GetStorageInfo (Variables|Default|Getlib) (Variables|Default|GetcontainerActor)))
        (if _cast_2
          (bind _sorted_storage_info_array (Default|SortStorageInfo _lib _overlayinfo (Variables|Default|GetsortType)))
          (Utilities|FlowControl|Sequence
            (:then_0
              (bind (_newparam1 _moreitems) (Default|StorageSlice _lib _sorted_storage_info_array (Variables|Default|GetshownItemsLength)))
              (for _array_element_2 _newparam1
                (bind _returnvalue_2 (UserInterface|CreateWidget "/Game/hbbtMod/Handables/smartphone/widgets/world/Storage/wg_containerInfoItem.wg_containerInfoItem_C" 0 _array_element_2))
                (Class|VerticalBox|AddChildtoVerticalBox (Variables|/Game/hbbtMod/Handables/smartphone/widgets/world/Storage/wg_containerInfo.wg_containerInfo_C|GetVerticalBox_70 (Variables|Default|GetContaionerInfo)) _returnvalue_2))
              (if (< 0 _moreitems)
                (bind _returnvalue_3 (UserInterface|CreateWidget "/Game/hbbtMod/Handables/smartphone/widgets/world/Storage/wg_containerInfoItemLast.wg_containerInfoItemLast_C" 0 (Utilities|Text|ToText(Integer) _moreitems)))
                (Class|VerticalBox|AddChildtoVerticalBox (Variables|/Game/hbbtMod/Handables/smartphone/widgets/world/Storage/wg_containerInfo.wg_containerInfo_C|GetVerticalBox_70 (Variables|Default|GetContaionerInfo)) _returnvalue_3)))
            (:then_1
              (Variables|Default|SetitemsGesamt 0)
              (for _array_element_3 _sorted_storage_info_array
                (bind _output_get (Variables|Default|SetitemsGesamt (+ (.ItemAmount (Utilities|Struct|Breakstruct_StorageInfo _array_element_3)) (Variables|Default|GetitemsGesamt))))
                (Rendering|Components|TextRender|SetText (Variables|/Game/hbbtMod/Handables/smartphone/widgets/world/Storage/wg_containerInfo.wg_containerInfo_C|GetTextBlock_itemAmount (Variables|Default|GetContaionerInfo)) (Utilities|Text|ToText(Integer) _output_get)))))
          (else
            (Class|SMLBlueprintLibrary|LogDebug "cant cast destroy actor -----------" true))))
      (:NewEnumerator2
        ;[1 1 1] Comment
        (Widget|Panel|ClearChildren (Variables|/Game/hbbtMod/Handables/smartphone/widgets/world/wg_MasterInfo.wg_MasterInfo_C|GetCanvasPanel_0 (Variables|Default|GetMasterWidget)))
        (bind _minerinfo (Default|GetMinerInfo (Variables|Default|Getlib) (Variables|Default|GetcontainerActor)))
        (bind _returnvalue_4 (UserInterface|CreateWidget "/Game/hbbtMod/Handables/smartphone/widgets/world/Miner/wg_MinerInfo.wg_MinerInfo_C" 0 _minerinfo))
        (Class|CanvasPanel|AddChildtoCanvas (Variables|/Game/hbbtMod/Handables/smartphone/widgets/world/wg_MasterInfo.wg_MasterInfo_C|GetCanvasPanel_0 (Variables|Default|GetMasterWidget)) _returnvalue_4))
      (:NewEnumerator3
        ;[1 1 1] Comment
        (Widget|Panel|ClearChildren (Variables|/Game/hbbtMod/Handables/smartphone/widgets/world/wg_MasterInfo.wg_MasterInfo_C|GetCanvasPanel_0 (Variables|Default|GetMasterWidget)))
        (bind _generator_info (Default|GetGeneratorInfo (Variables|Default|Getlib) (Variables|Default|GetcontainerActor)))
        (bind _returnvalue_5 (UserInterface|CreateWidget "/Game/hbbtMod/Handables/smartphone/widgets/world/Generator/wg_GeneratorInfo.wg_GeneratorInfo_C" 0 _generator_info))
        (Class|CanvasPanel|AddChildtoCanvas (Variables|/Game/hbbtMod/Handables/smartphone/widgets/world/wg_MasterInfo.wg_MasterInfo_C|GetCanvasPanel_0 (Variables|Default|GetMasterWidget)) _returnvalue_5)))))

(fn ConstructionScript)